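; End-of-level marker actor that ends the level when the player avatar enters its sphere.
; On overlap it pauses the avatar, removes its player UI and sets its state to stunned.
; It then blends the player camera to itself over a configurable time and, once the blend finishes, shows the Level_Complete widget.
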(event `self.Sphere.OnComponentBeginOverlap`
  (params (OverlappedComponent :type "PrimitiveComponent Object Reference") (OtherActor :type "Actor Object Reference") (OtherComp :type "PrimitiveComponent Object Reference") (OtherBodyIndex :type Integer) (bFromSweep :type Boolean) (SweepResult :type "HitResult Structure (by ref)"))
  (bind _time_to_transition_camera (`self.Time To Transition Camera`))
  (bind _asbp_avatar (cast `/Game/Blueprints/Characters_NPC_S/BP_Avatar` OtherActor))
  (if (== OtherActor _asbp_avatar)
    (set `Avatar.isPaused` true _asbp_avatar)
    (`Widget.RemoveFromParent` (`/Game/Blueprints/Characters_NPC_S/BP_Avatar.Player UI Reference` _asbp_avatar))
    (set `Avatar.currentState` "STUNNED" _asbp_avatar)
    (`PlayerController.SetViewTargetWithBlend` (`GameplayStatics.GetPlayerController` 0) self _time_to_transition_camera "VTBlend_Linear" 0.0 false)
    (`KismetSystemLibrary.Delay` _time_to_transition_camera)
    (bind _returnvalue (`|CreateWidget` "/Game/Blueprints/Widgets/Level_Complete.Level_Complete_C"))
    (`UserWidget.AddToViewport` _returnvalue 0)))

(fn `UserConstructionScript`)