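; Level tool Blueprint that shows and hides tutorial text in the player's dialogue UI.
; ShowTutorialText uses an integer index as the DataTable row name, then reveals the BP_Avatar UI's dialogue panel and fills in that row's Dialogue text.
; HideTutorialText hides the panel and the continue-dialogue image.
; Despite the collision name, the overlap event is disabled and nothing in this graph calls either event.
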(event `self.ShowTutorialText`
  (bind _returnvalue (`|GetDataTableRow` (`self.Data Table Reference`) (`KismetStringLibrary.Conv_StringToName` (`KismetStringLibrary.Conv_IntToString` (`self.indexOfDataTable`))))
    (:`then`
      (bind _asbp_avatar (cast `/Game/Blueprints/Characters_NPC_S/BP_Avatar` (`self.player`)))
      (bind _player_ui_reference (`/Game/Blueprints/Characters_NPC_S/BP_Avatar.Player UI Reference` _asbp_avatar))
      (`Widget.SetVisibility` (`/Game/Blueprints/Widgets/Player_UI.DialogePanel` _player_ui_reference) "Visible")
      (`TextBlock.SetText` (`/Game/Blueprints/Widgets/Player_UI.DialogueBoxText` _player_ui_reference) (`.Dialogue_6_3EC185AE438C26414FB2C4A83AB907FC` (break `/Game/Blueprints/Level_Tools/Data_Tables/Dialogue_Struct` _returnvalue))))))

(event `self.HideTutorialText`
  (bind _asbp_avatar (cast `/Game/Blueprints/Characters_NPC_S/BP_Avatar` (`self.player`)))
  (bind _player_ui_reference (`/Game/Blueprints/Characters_NPC_S/BP_Avatar.Player UI Reference` _asbp_avatar))
  (`Widget.SetVisibility` (`/Game/Blueprints/Widgets/Player_UI.DialogePanel` _player_ui_reference) "Hidden")
  (`Widget.SetVisibility` (`/Game/Blueprints/Widgets/Player_UI.ContinueDialogImage` _player_ui_reference) "Hidden"))

(fn `UserConstructionScript`)