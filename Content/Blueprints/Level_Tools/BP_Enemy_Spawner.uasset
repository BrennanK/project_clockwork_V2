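; Level-placed enemy spawner that calls SpawnEnemy once, the first time BP_Avatar overlaps its trigger box.
; BeginPlay sets the spawn point from the actor's location plus a MovableVector offset.
; SetPotentialPatrolPath hands the spawner's Path to a spawned actor if it is a BP_Patrolling_Enemy.
; The SpawnEnemy logic itself is not defined in these graphs.
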(event `self.ReceiveBeginPlay`
  (set `self.spawnPoint` (+ (`self.K2_GetActorLocation`) (`self.Movable Vector`))))

(event `self.Box.OnComponentBeginOverlap`
  (params (OverlappedComponent :type "PrimitiveComponent Object Reference") (OtherActor :type "Actor Object Reference") (OtherComp :type "PrimitiveComponent Object Reference") (OtherBodyIndex :type Integer) (bFromSweep :type Boolean) (SweepResult :type "HitResult Structure (by ref)"))
  (if (not (`self.initialEnemySpawned`))
    (cast `/Game/Blueprints/Characters_NPC_S/BP_Avatar` OtherActor)
    (`self.SpawnEnemy`)
    (set `self.initialEnemySpawned` true)))

(event `self.setPotentialPatrolPath`
  (params (spawn :type "Patrolling_Enemy Object Reference"))
  (bind _asbp_patrolling_enemy (cast `/Game/Blueprints/AI/BP_Patrolling_Enemy` spawn))
  (set `/Game/Blueprints/AI/BP_Patrolling_Enemy.Patrol_Path` (`self.Path`) _asbp_patrolling_enemy))

(fn `UserConstructionScript`)