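; Behavior Tree task that sets the next patrol destination for a BP_Patrolling_Enemy.
; It reads the current point index from the blackboard, picks that entry in the enemy's PatrolPath points, and adds the path actor's location.
; The resulting position is written to the blackboard vector key and the task finishes successfully.
; If the cast fails or the path is invalid, FinishExecute is never called.
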(event `self.ReceiveExecuteAI`
  (params (OwnerController :type "AIController Object Reference") (ControlledPawn :type "Pawn Object Reference"))
  (bind _asbp_patrolling_enemy (cast `/Game/Blueprints/AI/BP_Patrolling_Enemy` ControlledPawn))
  (bind _patrol_path (`/Game/Blueprints/AI/BP_Patrolling_Enemy.Patrol_Path` _asbp_patrolling_enemy)
    (:`then`
      (`BTFunctionLibrary.SetBlackboardValueAsVector` (`self.BB_PathVector`) (+ (`Actor.K2_GetActorLocation` _patrol_path) (`|GetArrayItem` (`/Game/Blueprints/AI/BP_PatrolPath.BP_Editable_Path+Points` _patrol_path) (`BTFunctionLibrary.GetBlackboardValueAsInt` (`self.BB_PathInt`)))))
      (`self.FinishExecute` true))
    (:`else`)))