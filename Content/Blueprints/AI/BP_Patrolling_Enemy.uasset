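; Patrolling enemy character with self-destruct feedback: blinking materials plus fuse and explosion sounds.
; BeginPlay seeds the Blackboard with its patrol path's looping flag, direction and wait time, taking the path from BP_Enemy_Spawner when respawnable.
; Custom events swap in self-destruct materials, raise the blink speed on body and chest dynamic material instances, and control audio.
; The fuse ignition sound hands off to a continuous burn after its duration.
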(event `self.ReceiveBeginPlay`
  (bind _returnvalue (`AIBlueprintHelperLibrary.GetBlackboard` null))
  (if (`self.isRespawnable`)
    (bind _asbp_enemy_spawner (cast `/Game/Blueprints/Level_Tools/BP_Enemy_Spawner` (`self.spawner`)))
    (set `self.Patrol_Path` (`/Game/Blueprints/Level_Tools/BP_Enemy_Spawner.Path` _asbp_enemy_spawner)))
  (`BlackboardComponent.SetValueAsBool` _returnvalue "PathLooping" (`/Game/Blueprints/AI/BP_PatrolPath.isLooping` (`self.Patrol_Path`)))
  (`BlackboardComponent.SetValueAsInt` _returnvalue "Direction" 1)
  (`BlackboardComponent.SetValueAsFloat` (`AIBlueprintHelperLibrary.GetBlackboard` null) "WaitTime" (`/Game/Blueprints/AI/BP_PatrolPath.Time Between Points` (`self.Patrol_Path`))))

(event `self.changeToSelfDestructMaterial`
  (bind _mesh (`self.Mesh`))
  (bind _mesh_2 (`self.Mesh`))
  (`PrimitiveComponent.SetMaterial` _mesh_2 0 "/Game/Self_Materials/Materials/Self_Destruct_Material.Self_Destruct_Material")
  (bind _returnvalue (`PrimitiveComponent.CreateDynamicMaterialInstance` _mesh_2 0 "/Game/Self_Materials/Materials/Patrolling_Enemy_Mat.Patrolling_Enemy_Mat" "None"))
  (bind _output_get (set `self.Body_Mat_Inst` _returnvalue))
  (`MaterialInstanceDynamic.SetScalarParameterValue` _output_get "Speed" (`self.slowBlinkSpeed`))
  (`PrimitiveComponent.SetMaterial` _mesh 1 "/Game/Self_Materials/Materials/Patrolling_Enemy_Mat.Patrolling_Enemy_Mat")
  (bind _returnvalue_2 (`PrimitiveComponent.CreateDynamicMaterialInstance` _mesh 1 "/Game/Self_Materials/Materials/Patrolling_Enemy_Mat.Patrolling_Enemy_Mat" "None"))
  (bind _output_get_2 (set `self.Chest_Mat_Inst` _returnvalue_2))
  (`MaterialInstanceDynamic.SetScalarParameterValue` _output_get_2 "Speed" (`self.slowBlinkSpeed`)))

(event `self.changeSpeedOfBlink`
  (`MaterialInstanceDynamic.SetScalarParameterValue` (`self.Body_Mat_Inst`) "Speed" (`self.fastBlinkSpeed`))
  (`MaterialInstanceDynamic.SetScalarParameterValue` (`self.Chest_Mat_Inst`) "Speed" (`self.fastBlinkSpeed`))
  (`KismetSystemLibrary.PrintString` "Fast Speed change got called" true true (struct :`G` 0.66 :`B` 1.0 :`A` 1.0) 6.0))

(event `self.playFuseLightSound`
  (bind _patrolling_enemy_audio_component (`self.Patrolling Enemy Audio Component`))
  (`AudioComponent.SetSound` _patrolling_enemy_audio_component "/Game/StarterContent/Audio/Externally_Imported_Sounds/Fuse_Light_Start.Fuse_Light_Start")
  (`AudioComponent.Play` _patrolling_enemy_audio_component 0.0)
  (`KismetSystemLibrary.Delay` (`SoundBase.Duration` (`AudioComponent.Sound` _patrolling_enemy_audio_component)))
  (`AudioComponent.SetSound` _patrolling_enemy_audio_component "/Game/StarterContent/Audio/Externally_Imported_Sounds/Lit_fuse_continuous.Lit_fuse_continuous")
  (`AudioComponent.Play` _patrolling_enemy_audio_component 0.0))

(event `self.playExplosionSound`
  (bind _patrolling_enemy_audio_component (`self.Patrolling Enemy Audio Component`))
  (`AudioComponent.SetSound` _patrolling_enemy_audio_component "/Game/StarterContent/Audio/Externally_Imported_Sounds/Patrol_Enemy_Explosion_Sound.Patrol_Enemy_Explosion_Sound")
  (`AudioComponent.Play` _patrolling_enemy_audio_component 0.0))

(event `self.stopFuseLightSound`
  (`AudioComponent.Stop` (`self.Patrolling Enemy Audio Component`)))

(fn `UserConstructionScript`
  (bind _mesh (`self.Mesh`))
  (bind _returnvalue (`PrimitiveComponent.CreateDynamicMaterialInstance` _mesh 0 "/Game/Self_Materials/Materials/Demonslayer_SP.Demonslayer_SP" "None"))
  (set `self.Body_Mat_Inst` _returnvalue)
  (bind _returnvalue_2 (`PrimitiveComponent.CreateDynamicMaterialInstance` _mesh 1 "/Game/Self_Materials/Materials/Demonslayer_SP.Demonslayer_SP" "None"))
  (set `self.Chest_Mat_Inst` _returnvalue_2)
  (set `self.skeleton` (`self.Mesh`))
  (set `self.capsuleCollider` (`self.CapsuleComponent`))
  (if (`self.isRespawnable`)
    (bind _asbp_enemy_spawner (cast `/Game/Blueprints/Level_Tools/BP_Enemy_Spawner` (`self.spawner`)))
    (set `self.Patrol_Path` (`/Game/Blueprints/Level_Tools/BP_Enemy_Spawner.Path` _asbp_enemy_spawner))))