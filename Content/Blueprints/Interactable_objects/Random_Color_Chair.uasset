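; An interactable chair actor that changes its seat color to a random one when the player walks into its trigger box.
; The construction script creates a dynamic material instance on the chair mesh's first material slot and stores it.
; On box overlap by the first player's pawn, it sets the ColorSeats vector parameter to a random RGB value.
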(event `self.Box.OnComponentBeginOverlap`
  (params (OverlappedComponent :type "PrimitiveComponent Object Reference") (OtherActor :type "Actor Object Reference") (OtherComp :type "PrimitiveComponent Object Reference") (OtherBodyIndex :type Integer) (bFromSweep :type Boolean) (SweepResult :type "HitResult Structure (by ref)"))
  (if (== OtherActor (`GameplayStatics.GetPlayerPawn` 0))
    (`MaterialInstanceDynamic.SetVectorParameterValue` (`self.Chair_Material_Instance`) "ColorSeats" (make `LinearColor` (`KismetMathLibrary.RandomFloatInRange` 0.0 1.0) (`KismetMathLibrary.RandomFloatInRange` 0.0 1.0) (`KismetMathLibrary.RandomFloatInRange` 0.0 1.0)))))

(fn `UserConstructionScript`
  (bind _returnvalue (`PrimitiveComponent.CreateDynamicMaterialInstance` (`self.SM_Chair`) 0 null "None"))
  (set `self.Chair_Material_Instance` _returnvalue))