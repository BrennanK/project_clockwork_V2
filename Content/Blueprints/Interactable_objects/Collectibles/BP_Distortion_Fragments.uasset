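; Collectible Distortion Fragments actor made of three fragment pieces, tinted according to its fragment value.
; The construction script creates a dynamic material instance for each piece.
; On BeginPlay, FragmentValue is converted to a row name to look up ColorTable, and the row's color sets ColorBase on all three materials.
; This graph handles appearance only and contains no pickup logic.
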(event `self.ReceiveBeginPlay`
  (bind _returnvalue (`|GetDataTableRow` (`self.Color_table`) (`KismetStringLibrary.Conv_StringToName` (`KismetStringLibrary.Conv_IntToString` (`self.fragmentValue`))))
    (:`then`
      (bind _color_of_fragment (break `/Game/Blueprints/Level_Tools/Data_Tables/Color_Scheme` _returnvalue))
      (`MaterialInstanceDynamic.SetVectorParameterValue` (`self.Dynamic_Frag_1_Mat`) "ColorBase" _color_of_fragment)
      (`MaterialInstanceDynamic.SetVectorParameterValue` (`self.Dynamic_Frag_2_Mat`) "ColorBase" _color_of_fragment)
      (`MaterialInstanceDynamic.SetVectorParameterValue` (`self.Dynamic_Frag_3_Mat`) "ColorBase" _color_of_fragment))))

(fn `UserConstructionScript`
  (bind _returnvalue (`PrimitiveComponent.CreateDynamicMaterialInstance` (`self.Frag 1`) 0 null "None"))
  (set `self.Dynamic_Frag_1_Mat` _returnvalue)
  (bind _returnvalue_2 (`PrimitiveComponent.CreateDynamicMaterialInstance` (`self.Frag 2`) 0 null "None"))
  (set `self.Dynamic_Frag_2_Mat` _returnvalue_2)
  (bind _returnvalue_3 (`PrimitiveComponent.CreateDynamicMaterialInstance` (`self.Frag 3`) 0 null "None"))
  (set `self.Dynamic_Frag_3_Mat` _returnvalue_3))