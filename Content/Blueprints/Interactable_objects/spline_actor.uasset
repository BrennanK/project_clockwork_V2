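; Spline actor that builds a deformed mesh along an editable spline, with a configurable static mesh and forward axis.
; The construction script adds one spline mesh component per segment, fitted to neighboring points' local positions and tangents, with query-only collision.
; An overlap event bound to the spline component prints a debug "Player hit spline" message for any actor, as the player-pawn check is unconnected.
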(event `self.Spline.OnComponentBeginOverlap`
  (params (OverlappedComponent :type "PrimitiveComponent Object Reference") (OtherActor :type "Actor Object Reference") (OtherComp :type "PrimitiveComponent Object Reference") (OtherBodyIndex :type Integer) (bFromSweep :type Boolean) (SweepResult :type "HitResult Structure (by ref)"))
  (`KismetSystemLibrary.PrintString` "Player hit spline"))

(fn `UserConstructionScript`
  (bind _spline (`self.Spline`))
  (for _index (range (+ (- (`SplineComponent.GetNumberOfSplinePoints` _spline) 2) 1))
    (bind _returnvalue (`AddComponent|NODE_AddSplineMeshComponent-0`))
    (`StaticMeshComponent.SetStaticMesh` _returnvalue (`self.Static Mesh of Spline`))
    (`SplineMeshComponent.SetForwardAxis` _returnvalue (`self.Spline Forward Axis`) true)
    (`SceneComponent.K2_AttachToComponent` _returnvalue (`self.Spline`) "None" "KeepRelative" "KeepRelative" "KeepRelative" true)
    (bind _returnvalue_2 (+ _index 1))
    (`SplineMeshComponent.SetStartAndEnd` _returnvalue (`SplineComponent.GetLocationAtSplinePoint` _spline _index "Local") (`SplineComponent.GetTangentAtSplinePoint` _spline _index "Local") (`SplineComponent.GetLocationAtSplinePoint` _spline _returnvalue_2 "Local") (`SplineComponent.GetTangentAtSplinePoint` _spline _returnvalue_2 "Local") true)
    (`PrimitiveComponent.SetCollisionEnabled` _returnvalue "QueryOnly")))