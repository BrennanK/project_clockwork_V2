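; Lock-on target actor for platforming that shows its targeting state through the color of its mesh.
; The construction script creates a dynamic material instance on the static mesh.
; Events for lock, unlock, indicate and reverse set its Color parameter, with ReverseLock restoring the same yellow as Lockon.
; BeginPlay copies the editable offset into VectorOffset, which is not used within this Blueprint.
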(event `self.ReceiveBeginPlay`
  (set `self.VectorOffset` (`self.Editable Offset`)))

(event `self.LockOn`
  (`MaterialInstanceDynamic.SetVectorParameterValue` (`self.Lock On Material Instance`) "Color" (struct :`R` 1.0 :`G` 0.9625 :`A` 1.0)))

(event `self.LockOff`
  (`MaterialInstanceDynamic.SetVectorParameterValue` (`self.Lock On Material Instance`) "Color" (struct :`R` 0.811765 :`G` 0.788235 :`B` 0.654902 :`A` 1.0)))

(event `self.indicateLock`
  (`MaterialInstanceDynamic.SetVectorParameterValue` (`self.Lock On Material Instance`) "Color" (struct :`G` 0.012961 :`B` 0.677083 :`A` 1.0)))

(event `self.reverseLock`
  (`MaterialInstanceDynamic.SetVectorParameterValue` (`self.Lock On Material Instance`) "Color" (struct :`R` 1.0 :`G` 0.9625 :`A` 1.0)))

(fn `UserConstructionScript`
  (bind _returnvalue (`PrimitiveComponent.CreateDynamicMaterialInstance` (`self.StaticMesh`) 0 null "None"))
  (set `self.Lock On Material Instance` _returnvalue))