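; Floor switch puzzle piece whose panel can turn green and play a color-change sound.
; The construction script creates and stores a dynamic material instance on the mesh's first material slot.
; Custom events set that instance's two emissive color parameters to green and play the switch audio component, as separate actions.
; It has no active overlap or trigger logic, and neither event is called within this Blueprint.
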(event `self.changePanelColorToGreen`
  (`MaterialInstanceDynamic.SetVectorParameterValue` (`self.Dynamic floor switch material`) "Emissive color 01" (struct :`R` 0.011599 :`G` 0.098958 :`B` 0.003492 :`A` 1.0))
  (`MaterialInstanceDynamic.SetVectorParameterValue` (`self.Dynamic floor switch material`) "Emissive color 02" (struct :`R` 0.023497 :`G` 1.0 :`B` 0.083553 :`A` 1.0)))

(event `self.playSwitchChangeColorSound`
  (`AudioComponent.Play` (`self.Switch Audio Component`) 0.0))

(fn `UserConstructionScript`
  (bind _returnvalue (`PrimitiveComponent.CreateDynamicMaterialInstance` (`self.Mesh`) 0 "/Game/Self_Materials/Materials/Floor_Switch_Test_Material.Floor_Switch_Test_Material" "None"))
  (set `self.Dynamic floor switch material` _returnvalue))