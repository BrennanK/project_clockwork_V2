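; Interactable puzzle-piece actor that toggles the interaction prompt on the player's UI.
; Its DisplayInteractionIcon and HideInteractionIcon events cast player character 0 to BP_Avatar and set the InteractionImage in its PlayerUIReference to Visible or Hidden.
; It holds no overlap, tick or interaction logic of its own, so both events depend on being called from elsewhere.
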(event `self.displayInteractionIcon`
  (bind _asbp_avatar (cast `/Game/Blueprints/Characters_NPC_S/BP_Avatar` (`GameplayStatics.GetPlayerCharacter` 0)))
  (`Widget.SetVisibility` (`/Game/Blueprints/Widgets/Player_UI.InteractionImage` (`/Game/Blueprints/Characters_NPC_S/BP_Avatar.Player UI Reference` _asbp_avatar)) "Visible"))

(event `self.hideInteractionIcon`
  (bind _asbp_avatar (cast `/Game/Blueprints/Characters_NPC_S/BP_Avatar` (`GameplayStatics.GetPlayerCharacter` 0)))
  (`Widget.SetVisibility` (`/Game/Blueprints/Widgets/Player_UI.InteractionImage` (`/Game/Blueprints/Characters_NPC_S/BP_Avatar.Player UI Reference` _asbp_avatar)) "Hidden"))

(fn `UserConstructionScript`)