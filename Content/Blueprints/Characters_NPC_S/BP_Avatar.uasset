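; Player avatar Blueprint handling HUD, pause menu, death fade, material states and sound for a character with punching, rail grinding and energy powers.
; Construction attaches hand spheres to sockets and caches component references; BeginPlay creates the player UI, which custom events update for health, energy and collectables.
; Helpers swap both mesh materials and play indexed sounds, while grinding chains start and continue sounds.
; Both punch-collision branches set PhysicsOnly, and rail-overlap spline logic is disconnected.
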(event `self.ReceiveBeginPlay`
  (set `self.playerCamera` (`self.Camera`))
  (set `self.isPunching` false)
  (set `self.capsuleA` (`self.CapsuleComponent`))
  (bind _returnvalue (`|CreateWidget` "/Game/Blueprints/Widgets/Player_UI.Player_UI_C" (`GameplayStatics.GetPlayerController` 0)))
  (`UserWidget.AddToViewport` _returnvalue 0)
  (set `self.Player UI Reference` _returnvalue))

(event `self.ReceiveTick`
  (params (DeltaSeconds :type "Float (single-precision)")))

(event `self.enableAndDisableCollision`
  (bind _lefthandsphere (`self.leftHandSphere`))
  (if (`self.isPunching`)
    (`PrimitiveComponent.SetCollisionEnabled` _lefthandsphere "PhysicsOnly")
    (`PrimitiveComponent.SetCollisionEnabled` (`self.rightHandSphere`) "PhysicsOnly")
    (else
      (`PrimitiveComponent.SetCollisionEnabled` _lefthandsphere "PhysicsOnly")
      (`PrimitiveComponent.SetCollisionEnabled` (`self.rightHandSphere`) "PhysicsOnly"))))

(event `self.Rail Collider.OnComponentBeginOverlap`
  (params (OverlappedComponent :type "PrimitiveComponent Object Reference") (OtherActor :type "Actor Object Reference") (OtherComp :type "PrimitiveComponent Object Reference") (OtherBodyIndex :type Integer) (bFromSweep :type Boolean) (SweepResult :type "HitResult Structure (by ref)")))

(event `self.callWheelChange`
  (`/Game/Blueprints/Widgets/Player_UI.Change Health Wheel Image` (`self.Player UI Reference`) (/ (`self.currentHealth`) (`self.maxHealth`))))

(event `self.callEnergyBarChange`
  (`/Game/Blueprints/Widgets/Player_UI.Change enrgy amount in Bar` (`self.Player UI Reference`) (/ (`self.currentEnergy`) (`self.maxEnergy`))))

(event `InputAction|Pause_game`
  (params (Key :type "Key Structure"))
  (bind _returnvalue (`GameplayStatics.GetPlayerController` 0))
  (:`Pressed`
    (if (not (`self.isPaused`))
      (bind _returnvalue_2 (`|CreateWidget` "/Game/Blueprints/Widgets/Pause_menu.Pause_menu_C"))
      (set `self.Pause Menu` _returnvalue_2)
      (`UserWidget.AddToViewport` _returnvalue_2 0)
      (set `self.isPaused` true)
      (`GameplayStatics.SetGamePaused` true)
      (`WidgetBlueprintLibrary.SetInputMode_UIOnlyEx` _returnvalue (`/Game/Blueprints/Widgets/Pause_menu.Resume_Button` _returnvalue_2))
      (set `PlayerController.bShowMouseCursor` true _returnvalue))))

(event `Reset Pause Variable`
  (set `self.isPaused` false))

(event `self.showCollectables`
  (bind _player_ui_reference (`self.Player UI Reference`))
  (if (`/Game/Blueprints/Widgets/Player_UI.All_Collectables Showing` _player_ui_reference)
    (`/Game/Blueprints/Widgets/Player_UI.hideAllCollectableUI` _player_ui_reference)
    (else
      (`/Game/Blueprints/Widgets/Player_UI.displayAllCollectibelUI` _player_ui_reference))))

(event `self.changeTimePowers`
  (if (not (`self.Time Powers Shown?`))
    (bind _returnvalue (`|CreateWidget` "/Game/Blueprints/Widgets/mainHUD.mainHUD_C"))
    (`UserWidget.AddToViewport` _returnvalue 0)))

(event `self.changeToEnergyMaterial`
  (`self.Alter Material` "/Game/Third_Person_FBX/M_Character_Energy_gain.M_Character_Energy_gain"))

(event `self.changeToAccelMaterial`
  (`self.Alter Material` "/Game/Third_Person_FBX/M_Character_Accel.M_Character_Accel"))

(event `self.changeToWarpMaterial`
  (`self.Alter Material` "/Game/Third_Person_FBX/M_Character_Warp.M_Character_Warp"))

(event `self.changeToNormalMaterial`
  (`self.Alter Material` "/Game/Third_Person_FBX/M_Character_Norm.M_Character_Norm"))

(event `self.activatePlayerActionSound`
  (params (indexOfSound :type Integer))
  (`self.Play Sound fromArray` indexOfSound (`self.Player Action Sound Component`)))

(event `self.activateGrindSound`
  (bind _player_mechanic_sound_component (`self.Player Mechanic Sound Component`))
  (`AudioComponent.SetSound` _player_mechanic_sound_component "/Game/StarterContent/Audio/Externally_Imported_Sounds/Rail_Grind_begin_sound.Rail_Grind_begin_sound")
  (`AudioComponent.Play` _player_mechanic_sound_component 0.0)
  (`KismetSystemLibrary.Delay` (`SoundBase.Duration` (`AudioComponent.Sound` _player_mechanic_sound_component)))
  (if (`self.isGrinding`)
    (`AudioComponent.SetSound` _player_mechanic_sound_component "/Game/StarterContent/Audio/Externally_Imported_Sounds/Continue_Grind_Sound.Continue_Grind_Sound")
    (`AudioComponent.Play` _player_mechanic_sound_component 0.0)))

(event `self.deactivateGrindSound`
  (`AudioComponent.Stop` (`self.Player Mechanic Sound Component`)))

(event `self.activateSoundFromDestroyedActor`
  (params (indexOfSound :type Integer))
  (`self.Play Sound fromArray` indexOfSound (`self.Destroyed Actor Sounds`)))

(event `self.playDeathFade`
  (bind _returnvalue (`|CreateWidget` "/Game/Blueprints/Widgets/Death_Widget.Death_Widget_C"))
  (`UserWidget.AddToViewport` _returnvalue 0))

(fn `Alter Material`
  (params (NewParam :type "Material Object Reference"))
  (bind _mesh (`self.Mesh`))
  (`PrimitiveComponent.SetMaterial` _mesh 0 NewParam)
  (`PrimitiveComponent.SetMaterial` _mesh 1 NewParam))

(fn `Play Sound fromArray`
  (params (`index Of Sound` :type Integer) (`Audio Component to Use` :type "AudioComponent Object Reference"))
  (`AudioComponent.SetSound` `Audio Component to Use` (`|GetArrayItem` (`self.Sound array`) `index Of Sound`))
  (`AudioComponent.Play` `Audio Component to Use` 0.0))

(fn `UserConstructionScript`
  (bind _mesh (`self.Mesh`))
  (bind _mesh_2 (`self.Mesh`))
  (`SceneComponent.K2_AttachToComponent` (`self.leftHandSphere`) _mesh "hand_l" "SnapToTarget" "KeepWorld" "KeepWorld" true)
  (`SceneComponent.K2_AttachToComponent` (`self.rightHandSphere`) _mesh "hand_r" "SnapToTarget" "KeepWorld" "KeepWorld" true)
  (set `self.skeleton` (`self.Mesh`))
  (set `self.teleportationParticle` (`self.Teleporter effect`))
  (set `self.cameraBoom` (`self.Camera Boom`))
  (bind _returnvalue (`PrimitiveComponent.CreateDynamicMaterialInstance` _mesh_2 0 null "None"))
  (set `self.Body_Material_Ref` _returnvalue)
  (bind _returnvalue_2 (`PrimitiveComponent.CreateDynamicMaterialInstance` _mesh_2 1 null "None"))
  (set `self.Chest_Material_Ref` _returnvalue_2))